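; Melee attack Gameplay Ability that plays a random attack montage from its avatar and damages nearby live players.
; On activation it sends a facing update using the combat target's location, then waits for a montage-tag gameplay event.
; That event's tag selects the combat socket centring a small radius damage check, after which the ability ends.
; Montage and awaited tag use separate random index expressions, so they can differ.
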(event Ability|EventActivateAbility
  (bind _returnvalue (Ability|GetAvatarActorfromActorInfo))
  (bind _returnvalue_2 (Class|EnemyInterface|GetCombatTarget(Message) (Ability|GetAvatarActorfromActorInfo)))
  (Class|CombatInterface|UpdateFacingTarget(Message) _returnvalue_2 (Transformation|GetActorLocation _returnvalue_2))
  (bind _returnvalue_3 (Class|CombatInterface|GetAttackMonatages(Message) (Ability|GetAvatarActorfromActorInfo)))
  (if (> (Utilities|Array|Length _returnvalue_3) 0)
    (|PlayMontageandWaitProxy "None" (.Montage (Utilities|Struct|BreakTaggedMontage (Utilities|Array|Get(acopy) _returnvalue_3 (Math|Random|RandomIntegerinRange 0 (- (Utilities|Array|Length _returnvalue_3) 1))))) 1.0 "None" true 1.0 0.0 false
      (:then
        (bind _payload (Ability|Tasks|WaitGameplayEvent (.MontageTag (Utilities|Struct|BreakTaggedMontage (Utilities|Array|Get(acopy) _returnvalue_3 (Math|Random|RandomIntegerinRange 0 (- (Utilities|Array|Length _returnvalue_3) 1))))) 0)
          (:EventReceived
            (bind _returnvalue_4 (Class|CombatInterface|GetCombatSocketLocation(Message) (Ability|GetAvatarActorfromActorInfo) (.EventTag (Utilities|Struct|BreakGameplayEventData _payload))))
            (bind _outoverlappingactors (Class|AuraAbilitySystemLibrary|GetLivePlayersWithinRadius _returnvalue (Utilities|Array|MakeArray _returnvalue) 45.0 _returnvalue_4))
            (for _array_element _outoverlappingactors
              (Class|AuraDamageGameplayAbility|CauseDamage _array_element))
            (Ability|EndAbility)))))
    (else
      (Ability|EndAbility))))

(event Ability|EventOnEndAbility
  (params (bWasCancelled :type Boolean)))