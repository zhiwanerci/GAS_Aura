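; GA_MeleeAttack is an enemy gameplay ability that performs a melee attack against the avatar's combat target.
; It turns the avatar toward the target, plays a random tagged montage and waits for that montage's gameplay event.
; On the event it sphere-queries live players around the montage's combat socket, damaging non-friends and triggering blood effects.
; Any hit fires a MeleeImpact gameplay cue at the socket, then the ability ends.
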(event Ability|EventActivateAbility
  (bind _returnvalue (Ability|GetAvatarActorfromActorInfo))
  (bind _returnvalue_2 (Ability|GetAvatarActorfromActorInfo))
  (bind _returnvalue_3 (Ability|GetAvatarActorfromActorInfo))
  (bind _returnvalue_4 (Class|EnemyInterface|GetCombatTarget(Message) _returnvalue_2))
  (Class|CombatInterface|UpdateFacingTarget(Message) _returnvalue_2 (Transformation|GetActorLocation _returnvalue_4))
  (bind _returnvalue_5 (Class|CombatInterface|GetAttackMonatages(Message) (Ability|GetAvatarActorfromActorInfo)))
  (Variables|Default|SetCurTagged (Class|AuraDamageGameplayAbility|GetRandomTaggedMontagefromArray _returnvalue_5))
  (if (> (Utilities|Array|Length _returnvalue_5) 0)
    (|PlayMontageandWaitProxy "None" (.Montage (Utilities|Struct|BreakTaggedMontage (Variables|Default|GetCurTagged))) 1.0 "None" false 1.0 0.0 false
      (:then
        (Ability|Tasks|WaitGameplayEvent (.MontageTag (Utilities|Struct|BreakTaggedMontage (Variables|Default|GetCurTagged))) 0
          (:EventReceived
            (bind _returnvalue_6 (Class|CombatInterface|GetCombatSocketLocation(Message) (Ability|GetAvatarActorfromActorInfo) (.SocketTag (Utilities|Struct|BreakTaggedMontage (Variables|Default|GetCurTagged)))))
            (Variables|Default|SetCombatSocketLocation _returnvalue_6)
            (bind _outoverlappingactors (Class|AuraAbilitySystemLibrary|GetLivePlayersWithinRadius _returnvalue_3 (Utilities|Array|MakeArray _returnvalue_3) 45.0 (Variables|Default|GetCombatSocketLocation)))
            (for _array_element _outoverlappingactors
              (if (Class|AuraAbilitySystemLibrary|IsNotFriend (Ability|GetAvatarActorfromActorInfo) _array_element)
                (Class|AuraDamageGameplayAbility|CauseDamage _array_element)
                (Variables|Default|SetHasHitTarget true)
                (Class|CombatInterface|GetBloodEffect(Message) _array_element)))
            (if (Variables|Default|GetHasHitTarget)
              (bind _returnvalue_7 (Class|EnemyInterface|GetCombatTarget(Message) _returnvalue))
              (Class|GameplayAbility|ExecuteGameplayCuewithParams "(TagName=\"GameplayCue.MeleeImpact\")" (Ability|GameplayCue|MakeGameplayCueParameters :AggregatedSourceTags (GameplayTags|MakeGameplayTagContainerfromTag (.MontageTag (Utilities|Struct|BreakTaggedMontage (Variables|Default|GetCurTagged)))) :Location (Variables|Default|GetCombatSocketLocation) :EffectCauser _returnvalue :SourceObject _returnvalue_7)))
            (Ability|EndAbility))))
      (:OnCompleted
        (Ability|EndAbility :!label _label))
      (:OnInterrupted
        (goto _label))
      (:OnCancelled
        (goto _label)))
    (else
      (Ability|EndAbility))))