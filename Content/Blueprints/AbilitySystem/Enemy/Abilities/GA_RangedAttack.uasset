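; Enemy gameplay ability for a ranged attack that fires a projectile at the avatar's combat target.
; On activation it turns the avatar toward the target and plays a random tagged attack montage.
; A gameplay event matching the montage's tag spawns the projectile from its socket tag toward the target's current location.
; The ability ends when the montage completes, is interrupted or cancelled, or when no montages exist.
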(event Ability|EventActivateAbility
  (bind _returnvalue (Ability|GetAvatarActorfromActorInfo))
  (bind _returnvalue_2 (Class|EnemyInterface|GetCombatTarget(Message) _returnvalue))
  (Class|CombatInterface|UpdateFacingTarget(Message) _returnvalue (Transformation|GetActorLocation _returnvalue_2))
  (bind _returnvalue_3 (Class|CombatInterface|GetAttackMonatages(Message) (Ability|GetAvatarActorfromActorInfo)))
  (Variables|Default|SetCurTagged (Class|AuraDamageGameplayAbility|GetRandomTaggedMontagefromArray _returnvalue_3))
  (if (> (Utilities|Array|Length _returnvalue_3) 0)
    (|PlayMontageandWaitProxy "None" (.Montage (Utilities|Struct|BreakTaggedMontage (Variables|Default|GetCurTagged))) 1.0 "None" false 1.0 0.0 false
      (:then
        (Ability|Tasks|WaitGameplayEvent (.MontageTag (Utilities|Struct|BreakTaggedMontage (Variables|Default|GetCurTagged))) 0
          (:EventReceived
            (bind _returnvalue_4 (Class|EnemyInterface|GetCombatTarget(Message) (Ability|GetAvatarActorfromActorInfo)))
            (Class|AuraProjectileSpell|SpawnProjectile (Transformation|GetActorLocation _returnvalue_4) (.SocketTag (Utilities|Struct|BreakTaggedMontage (Variables|Default|GetCurTagged)))))))
      (:OnCompleted
        (Ability|EndAbility :!label _label))
      (:OnInterrupted
        (goto _label))
      (:OnCancelled
        (goto _label)))
    (else
      (Ability|EndAbility))))

(event Ability|EventOnEndAbility
  (params (bWasCancelled :type Boolean)))